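; Voxel terrain chunk actor that builds blocky ground with scattered scenery around its location, only in the TEST level.
; The construction script loops a grid, offsets each column's height with world-space 2D simplex noise, and adds blocks as mesh instances.
; Random rolls place tree, rock, grass and flower instances at randomly picked recorded block positions.
; The trap roll is empty, and the tree-pickup spawning logic is unconnected.
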(event `self.ReceiveBeginPlay`)

(fn `UserConstructionScript`
  (bind _returnvalue (`KismetMathLibrary.RandomIntegerInRange` 0 100))
  (bind _returnvalue_2 (`KismetMathLibrary.RandomFloatInRange` 0.75 1.2))
  (bind _returnvalue_3 (`KismetMathLibrary.RandomFloatInRange` 1.0 1.5))
  (bind _returnvalue_4 (`KismetMathLibrary.RandomFloatInRange` 1.5 3.0))
  (bind _returnvalue_5 (`KismetMathLibrary.RandomFloatInRange` 0.4 0.5))
  (bind _num (`self.Num`))
  (bind _voxelsize (`self.VoxelSize`))
  (bind _num_2 (`self.Num`))
  (bind _depth (`self.Depth`))
  (bind _voxelsize_2 (`self.VoxelSize`))
  (bind (_outitem _outindex) (`KismetArrayLibrary.Array_Random` (`self.TreesCoordLists`)))
  (bind (_outitem_2 _outindex_2) (`KismetArrayLibrary.Array_Random` (`self.TreesCoordLists`)))
  (bind (_outitem_3 _outindex_3) (`KismetArrayLibrary.Array_Random` (`self.TreesCoordLists`)))
  (bind (_outitem_4 _outindex_4) (`KismetArrayLibrary.Array_Random` (`self.TreesCoordLists`)))
  (bind _returnvalue_6 (* (`self.WorldPosZ-PostNoise`) (`self.VoxelSize`)))
  (bind _returnvalue_7 (`KismetMathLibrary.MakeVector` (* (`self.LocalVoxelPosX`) _voxelsize_2) (* (`self.LocalVoxelPosY`) _voxelsize_2) _returnvalue_6))
  (bind _returnvalue_8 (`KismetMathLibrary.MakeTransform` (`KismetMathLibrary.MakeVector` (.x _outitem_3) (.y _outitem_3) (+ (.z _outitem_3) 47.5)) (struct) (`KismetMathLibrary.MakeVector` _returnvalue_3 _returnvalue_3 _returnvalue_3)))
  (bind _returnvalue_9 (`GameplayStatics.GetCurrentLevelName` true))
  (if (== _returnvalue_9 "TEST")
    ;[1 1 1] Loops
    (for _index (range (* _num -1) (+ _num 1))
      (set `self.LocalVoxelPosX` _index)
      (for _index_2 (range (* _num_2 -1) (+ _num_2 1))
        (set `self.LocalVoxelPosY` _index_2)
        (for _index_3 (range (* _depth -1) (+ _depth 1))
          (set `self.LocalVoxelPosZ` _index_3)
          ;[1 1 1] Set Voxel Coordinates
          (set `self.WorldVoxelPosX` (+ (`self.LocalVoxelPosX`) (`KismetMathLibrary.FFloor` (.x (/ (`self.K2_GetActorLocation`) (`self.VoxelSize`))))))
          (set `self.WorldVoxelPosY` (+ (`self.LocalVoxelPosY`) (`KismetMathLibrary.FFloor` (.y (/ (`self.K2_GetActorLocation`) (`self.VoxelSize`))))))
          (set `self.WorldVoxelPosZ` (+ (`self.LocalVoxelPosZ`) (`KismetMathLibrary.FFloor` (.z (/ (`self.K2_GetActorLocation`) (`self.VoxelSize`))))))
          ;[1 1 1] Calculate 2d Noise
          (bind _returnvalue_10 (`SimplexNoiseBPLibrary.SimplexNoise2D` (* (`self.WorldVoxelPosX`) _voxelsize) (* (`self.WorldVoxelPosY`) _voxelsize) (`self.NoiseDensity`)))
          (set `self.WorldPosZ-PostNoise` (- (`KismetMathLibrary.FFloor` (* (`self.NoiseScale`) _returnvalue_10)) (`self.LocalVoxelPosZ`)))
          ;[1 1 1] Add Block Instance
          (`KismetSystemLibrary.PrintString` (`KismetStringLibrary.Conv_DoubleToString` _returnvalue_6))
          (set `self.TreesCoord` _returnvalue_7)
          (`InstancedStaticMeshComponent.AddInstance` (`self.InstancedStaticMesh`) (`KismetMathLibrary.MakeTransform` _returnvalue_7 (struct) (* (1.0 1.0 1.0) (/ (`self.VoxelSize`) 100.0))) false)
          (`KismetArrayLibrary.Array_Add` (`self.TreesCoordLists`) (`self.TreesCoord`))
          (`|ExecutionSequence`
            (:`then_0`
              ;[1 1 1] Add Tree Instance
              (set `self.ChanceToSpawnTrees` _returnvalue)
              (if (>= _returnvalue 85)
                (`InstancedStaticMeshComponent.AddInstance` (`self.InstancedStaticMeshTree`) (`KismetMathLibrary.MakeTransform` (`KismetMathLibrary.MakeVector` (.x _outitem_2) (.y _outitem_2) (+ (.z _outitem_2) 47.0)) (struct) (`KismetMathLibrary.MakeVector` _returnvalue_2 _returnvalue_2 _returnvalue_2)) false)
                (set `self.Index_Coord_Tree` _outindex_2)
                (`KismetArrayLibrary.Array_Remove` (`self.TreesCoordLists`) (`self.Index_Coord_Tree`))))
            (:`then_1`
              ;[1 1 1] Add Rock Instance
              (if (>= (`KismetMathLibrary.RandomIntegerInRange` 0 100) 98)
                (`InstancedStaticMeshComponent.AddInstance` (`self.InstancedStaticMeshRock`) (`KismetMathLibrary.MakeTransform` (`KismetMathLibrary.MakeVector` (.x _outitem_4) (.y _outitem_4) (+ (.z _outitem_4) 47.0)) (struct) (`KismetMathLibrary.MakeVector` _returnvalue_5 _returnvalue_5 _returnvalue_5)) false)
                (set `self.IndexCoordStone` _outindex_4)
                (`KismetArrayLibrary.Array_Remove` (`self.TreesCoordLists`) (`self.IndexCoordStone`))))
            (:`then_2`
              (if (>= (`KismetMathLibrary.RandomIntegerInRange` 0 100) 80)
                (switch `int` (`KismetMathLibrary.RandomInteger` 3)
                  (:`0`
                    (`InstancedStaticMeshComponent.AddInstance` (`self.InstancedStaticMeshGrass`) _returnvalue_8 false))
                  (:`1`
                    (`InstancedStaticMeshComponent.AddInstance` (`self.InstancedStaticMeshGrass_2`) _returnvalue_8 false))
                  (:`2`
                    (`InstancedStaticMeshComponent.AddInstance` (`self.InstancedStaticMeshGrass_3`) _returnvalue_8 false)))
                (set `self.IndexCoordGrass` _outindex_3)
                (`KismetArrayLibrary.Array_Remove` (`self.TreesCoordLists`) (`self.IndexCoordStone`))))
            (:`then_3`
              ;[1 1 1] Add Flowers Instance
              (if (>= (`KismetMathLibrary.RandomFloatInRange` 0.0 100.0) 99.0)
                (`InstancedStaticMeshComponent.AddInstance` (`self.InstancedStaticMeshFlower`) (`KismetMathLibrary.MakeTransform` (`KismetMathLibrary.MakeVector` (.x _outitem) (.y _outitem) (+ (.z _outitem) 50.0)) (struct) (`KismetMathLibrary.MakeVector` _returnvalue_4 _returnvalue_4 _returnvalue_4)) false)
                (set `self.IndexCoordFlower` _outindex)
                (`KismetArrayLibrary.Array_Remove` (`self.TreesCoordLists`) (`self.IndexCoordFlower`))))
            (:`then_4`
              ;[1 1 1] Piege
              (if (>= (`KismetMathLibrary.RandomFloatInRange` 0.0 100.0) 99.0)
                _))))))))