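; Spawn_BP is a placement actor that scatters copies of ActorV01 over surfaces within a configurable box area.
; Its construction script sizes the Container box, then repeatedly line-traces downward from high above random points in it against chosen object types.
; Each hit adds a child actor component with random yaw, using the hit location as its relative transform.
; A Selection switch also sets the ChildActor component's class; the event graph is inactive.
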(event `self.ReceiveBeginPlay`)

(fn `UserConstructionScript`
  (bind (_origin _boxextent) (`KismetSystemLibrary.GetComponentBounds` (`self.Container`)))
  (bind _returnvalue (`KismetMathLibrary.MakeVector` (.x (`KismetMathLibrary.RandomPointInBoundingBox` _origin _boxextent)) (.y (`KismetMathLibrary.RandomPointInBoundingBox` _origin _boxextent)) (+ (.z (`KismetMathLibrary.RandomPointInBoundingBox` _origin _boxextent)) 100000.0)))
  (`|ExecutionSequence`
    (:`then_0`
      (switch `int` (`self.Selection`)
        (:`0`
          (`ChildActorComponent.SetChildActorClass` (`self.ChildActor`) (`self.ActorV01`)))))
    (:`then_1`
      (if (== (`self.In Box Extent`) (0.0 0.0 0.0))
        (set `self.In Box Extent` (0.0 0.0 0.0)))
      (`BoxComponent.SetBoxExtent` (`self.Container`) (`self.In Box Extent`) false)
      (for _ (range (`self.Last Index`))
        (bind (_outhit _returnvalue_2) (`KismetSystemLibrary.LineTraceSingleForObjects` _returnvalue (+ _returnvalue (* (* (`self.GetActorUpVector`) -1) 150000.0)) (`self.Object Types`)))
        (if _returnvalue_2
          (bind (_bblockinghit _binitialoverlap _time _distance _location) (`GameplayStatics.BreakHitResult` _outhit))
          (bind _returnvalue_3 (`AddComponent|NODE_AddChildActorComponent-2` :`RelativeTransform` (`KismetMathLibrary.MakeTransform` _location (`KismetMathLibrary.MakeRotator` 0.0 0.0 (`KismetMathLibrary.RandomFloatInRange` 0.0 (`self.MaxRotation`))))))
          (`ChildActorComponent.SetChildActorClass` _returnvalue_3 (`self.ActorV01`))
          (`KismetSystemLibrary.PrintString` (`KismetStringLibrary.Conv_BoolToString` _bblockinghit))
          (if (== _bblockinghit false)
            _))))))