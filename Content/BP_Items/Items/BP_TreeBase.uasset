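; BP_TreeBase is a tree item that the player harvests with the Pickup input while overlapping it.
; Begin and end overlap on its StaticMesh enable and disable input from player controller 0, so the key works only in range.
; On press, a loop counts Quantity down to zero, spawning one Actor-specified object at the player's location each pass, then destroys the tree.
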(event `InputAction|Pickup`
  (params (Key :type "Key Structure"))
  (bind (_returnvalue_x _returnvalue_y _returnvalue_z) (`KismetMathLibrary.BreakVector` (`self.K2_GetActorLocation` (`/Game/Essentiels.GET_PLAYER`))))
  (:`Pressed`
    (while (!= (`self.Quantity`) 0)
      (`/Engine/EditorBlueprintResources/StandardMacros.DecrementInt` (`self.Quantity`)
        (:`  `
          (`|SpawnActorFromClass` (`self.Actor`) (`KismetMathLibrary.MakeTransform` (`KismetMathLibrary.MakeVector` _returnvalue_x _returnvalue_y _returnvalue_z)) "Undefined" "OverrideRootScale" null null))))
    (`self.K2_DestroyActor`)))

(event `self.StaticMesh.OnComponentBeginOverlap`
  (params (OverlappedComponent :type "PrimitiveComponent Object Reference") (OtherActor :type "Actor Object Reference") (OtherComp :type "PrimitiveComponent Object Reference") (OtherBodyIndex :type Integer) (bFromSweep :type Boolean) (SweepResult :type "HitResult Structure (by ref)"))
  (`self.EnableInput` (`GameplayStatics.GetPlayerController` 0)))

(event `self.StaticMesh.OnComponentEndOverlap`
  (params (OverlappedComponent :type "PrimitiveComponent Object Reference") (OtherActor :type "Actor Object Reference") (OtherComp :type "PrimitiveComponent Object Reference") (OtherBodyIndex :type Integer))
  (`self.DisableInput` (`GameplayStatics.GetPlayerController` 0)))

(fn `UserConstructionScript`)