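; Base world pickup item that shows an info widget and lets the player collect it for EXP.
; Construction loads item data and mesh from a data table row; BeginPlay randomizes stacked quantities, may spawn Cobblestone for such Rock items, and fills the widget.
; Box overlap with BP_Player toggles the widget, input and a gate, so Pickup adds the item and destroys the actor.
; Tick repositions the widget whenever the box's rounded location changes.
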(event `self.ReceiveBeginPlay`
  (bind _information_ (`self.Information `))
  (bind (_name _types _description _icon _staticmesh _rarity _quantity) (break `/Game/Inventory_System/Structures/ST_Item` _information_))
  (if (>= _quantity 2)
    (setmembers `/Game/Inventory_System/Structures/ST_Item` :`StructRef` _information_ :`Quantity` (`KismetMathLibrary.RandomIntegerInRange` 1 _quantity))
    (`self.CheckIfGetOres`))
  (bind _asinteract_pickup_collect (cast `/Game/PickupSystems/Widget/Interact_Pickup_Collect` (`WidgetComponent.GetUserWidgetObject` (`self.Widget`))))
  (`|ExecutionSequence`
    (:`then_0`
      (`TextBlock.SetText` (`/Game/PickupSystems/Widget/Interact_Pickup_Collect.ItemTypeText` _asinteract_pickup_collect) (`KismetTextLibrary.Conv_StringToText` (`|GetEnumeratorNameAsString` (enumliteral `/Game/Inventory_System/Enum/Item_types` _types)))))
    (:`then_1`
      (`TextBlock.SetText` (`/Game/PickupSystems/Widget/Interact_Pickup_Collect.ItemNameText` _asinteract_pickup_collect) (`KismetTextLibrary.Conv_NameToText` _name)))
    (:`then_2`
      (`TextBlock.SetText` (`/Game/PickupSystems/Widget/Interact_Pickup_Collect.ItemQuantityText` _asinteract_pickup_collect) (`|FormatText` "Quantity: {Q}" _quantity)))))

(event `self.ReceiveTick`
  (params (DeltaSeconds :type "Float (single-precision)"))
  (bind (_x _y _z) (`self.GetBoxCoord`))
  (bind (_x_2 _y_2 _z_2) (`self.GetBoxCoord`))
  (bind (_lastknowsmcoord_x _lastknowsmcoord_y _lastknowsmcoord_z) (break `IntVector` (`self.LastKnowSMCoord`)))
  (bind (_lastknowsmcoord_x_2 _lastknowsmcoord_y_2 _lastknowsmcoord_z_2) (break `IntVector` (`self.LastKnowSMCoord`)))
  ;[1 1 1] re adapt widget information
  (if (not (and (== _x_2 _lastknowsmcoord_x_2) (== _y_2 _lastknowsmcoord_y_2) (== _z_2 _lastknowsmcoord_z_2)))
    (set `self.LastKnowSMCoord` (make `IntVector` _x _y _z))
    (`SceneComponent.K2_SetWorldLocation` (`self.Widget`) (`KismetMathLibrary.MakeVector` (`KismetMathLibrary.Conv_IntToDouble` _lastknowsmcoord_x) (`KismetMathLibrary.Conv_IntToDouble` _lastknowsmcoord_y) (`KismetMathLibrary.Conv_IntToDouble` _lastknowsmcoord_z)) false false)))

(event `InputAction|Pickup`
  (params (Key :type "Key Structure"))
  (:`Pressed`
    (`/Engine/EditorBlueprintResources/StandardMacros.Gate` true :!label _label
      (:`Exit`
        (bind _successadded (`/Game/Inventory_System/Libraries/BFL_Inventory.ItemToAdd` (`self.Information `) (`.Quantity_27_1BBDAB1940712B917E1F0C8BC6B92E5C` (break `/Game/Inventory_System/Structures/ST_Item` (`self.Information `)))))
        (if _successadded
          (`self.K2_DestroyActor`)
          (bind _asbp_player (cast `/Game/Character/BP_Player` (`GameplayStatics.GetPlayerCharacter` 0)))
          (`/Game/LevellingSystem.AddExp` (`/Game/Character/BP_Player.LevellingSystem` _asbp_player) (`.EXP_30_5DDC3A904AEBCF059C5F1BB9593CB7FA` (break `/Game/Inventory_System/Structures/ST_Item` (`self.Information `)))))))))

(event `self.Box.OnComponentBeginOverlap`
  (params (OverlappedComponent :type "PrimitiveComponent Object Reference") (OtherActor :type "Actor Object Reference") (OtherComp :type "PrimitiveComponent Object Reference") (OtherBodyIndex :type Integer) (bFromSweep :type Boolean) (SweepResult :type "HitResult Structure (by ref)"))
  (if (`KismetMathLibrary.ClassIsChildOf` (`GameplayStatics.GetObjectClass` OtherActor) "/Game/Character/BP_Player.BP_Player_C")
    (`SceneComponent.SetVisibility` (`self.Widget`) true false)
    (`self.EnableInput` (`GameplayStatics.GetPlayerController` 0))
    (goto _label :!via `Open`)))

(event `self.Box.OnComponentEndOverlap`
  (params (OverlappedComponent :type "PrimitiveComponent Object Reference") (OtherActor :type "Actor Object Reference") (OtherComp :type "PrimitiveComponent Object Reference") (OtherBodyIndex :type Integer))
  (if (`KismetMathLibrary.ClassIsChildOf` (`GameplayStatics.GetObjectClass` OtherActor) "/Game/Character/BP_Player.BP_Player_C")
    (`SceneComponent.SetVisibility` (`self.Widget`) false false)
    (`self.DisableInput` (`GameplayStatics.GetPlayerController` 0) null)
    (goto _label :!via `Close`)))

(fn `CheckIfGetOres`
  (bind (_returnvalue_x _returnvalue_y _returnvalue_z) (`KismetMathLibrary.BreakVector` (`SceneComponent.K2_GetComponentLocation` (`self.Box`))))
  (if (== (`.Actor_35_9AE228DF4D4C5D0BC3B7FD86F95A1FDE` (break `/Game/Inventory_System/Structures/ST_Item` (`self.Information `))) "/Game/BP_Items/Items/Rock.Rock_C")
    (if (>= (`KismetMathLibrary.RandomIntegerInRange` 0 100) 70)
      (`|SpawnActorFromClass` "/Game/BP_Items/Items/Cobblestone.Cobblestone_C" (`KismetMathLibrary.MakeTransform` (`KismetMathLibrary.MakeVector` _returnvalue_x _returnvalue_y (+ _returnvalue_z 30.0)) (struct) (0.4 0.4 0.4)) "Undefined" "OverrideRootScale" null null))))

(fn `GetBoxCoord`
  (returns (X :type Integer) (Y :type Integer) (Z :type Integer))
  (return (`KismetMathLibrary.Round` (.x (`SceneComponent.K2_GetComponentLocation` (`self.Box`)))) (`KismetMathLibrary.Round` (.y (`SceneComponent.K2_GetComponentLocation` (`self.Box`)))) (`KismetMathLibrary.Round` (.z (`SceneComponent.K2_GetComponentLocation` (`self.Box`))))))

(fn `SpawnOthersActors`
  (locals (QuantityItem :type Integer))
  (bind (_name _types _description _icon _staticmesh _rarity _quantity _stackable _exp _actor) (break `/Game/Inventory_System/Structures/ST_Item` (`self.Information `)))
  (set `local.QuantityItem` _quantity)
  (while (!= (`local.QuantityItem`) 0)
    (set `local.QuantityItem` (- (`local.QuantityItem`) 1))
    (`KismetSystemLibrary.PrintString` (`KismetStringLibrary.Conv_IntToString` (`local.QuantityItem`)))
    (`|SpawnActorFromClass` _actor (`KismetMathLibrary.MakeTransform` (0.0 0.0 0.0)) "Undefined" "OverrideRootScale" null null)))

(fn `UserConstructionScript`
  (bind (_datatable _rowname) (break `DataTableRowHandle` (`self.Item`)))
  (bind _returnvalue (`|GetDataTableRow` _datatable _rowname)
    (:`then`
      (set `self.Information ` _returnvalue)
      (`StaticMeshComponent.SetStaticMesh` (`self.StaticMesh`) (`.StaticMesh_18_73C195EF4D3F180B0155AA81DC2CE5CD` (break `/Game/Inventory_System/Structures/ST_Item` (`self.Information `)))))))